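; BP_P38 is a P-38 aircraft actor with two spinning propellers, Left and Right.
; On BeginPlay it registers both with its BPRotateSceneComponent, which by its name handles the rotation.
; A RotatePropeller function can roll a given component at PropellerRotationSpeed scaled by delta time, but nothing here calls it.
; Tick is empty, and a world-offset movement along X is left disconnected.
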(event `self.ReceiveBeginPlay`
  (`KismetArrayLibrary.Array_Add` (`/Game/Blueprints/BP_RotateSceneComponent.SceneComponents` (`self.BP_RotateSceneComponent`)) (`self.Left`))
  (`KismetArrayLibrary.Array_Add` (`/Game/Blueprints/BP_RotateSceneComponent.SceneComponents` (`self.BP_RotateSceneComponent`)) (`self.Right`)))

(event `self.ReceiveTick`
  (params (DeltaSeconds :type "Float (single-precision)")))

(fn `RotatePropeller`
  (params (Where :type "SceneComponent Object Reference"))
  (`SceneComponent.K2_AddLocalRotation` Where (`KismetMathLibrary.MakeRotator` (* (`GameplayStatics.GetWorldDeltaSeconds`) (`self.PropellerRotationSpeed`))) false false))

(fn `UserConstructionScript`)